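; BP_FadeActor is an actor whose mesh fades out and back in through a timeline-driven "Fade" material parameter.
; Construction caches the original materials and creates dynamic instances from FadeMaterialInstances.
; FadeOut swaps in those instances and plays the timeline, while Fadein reverses it.
; On finish, a value of 1 restores the originals; with BlockVisibility set, Visibility collision blocks at 1 and is ignored at 0.
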(event EventBeginPlay)

(event EventFadeOut
  (CallFunction|SetMaterialtoDynamicInstances)
  (bind _fade (Timeline|FadeTimeline Play)
    (:Update
      (for _array_element (Variables|Default|GetMaterialInstancesDynamic)
        (Rendering|Material|SetScalarParameterValue _array_element "Fade" _fade :!class /Script/Engine.MaterialInstanceDynamic)))
    (:Finished
      (CallFunction|FadeFinished _fade))))

(event EventFadein
  (bind _fade (Timeline|FadeTimeline Reverse)
    (:Update
      (for _array_element (Variables|Default|GetMaterialInstancesDynamic)
        (Rendering|Material|SetScalarParameterValue _array_element "Fade" _fade :!class /Script/Engine.MaterialInstanceDynamic)))
    (:Finished
      (CallFunction|FadeFinished _fade))))

(fn ConstructionScript
  (Utilities|Array|Clear (Variables|Default|GetMaterialInstancesDynamic))
  (Variables|Default|SetOriginalMaterials (Rendering|Material|GetMaterials (Variables|Default|GetMesh)))
  (for _array_element (Variables|Default|GetFadeMaterialInstances)
    (bind _returnvalue (Rendering|Material|CreateDynamicMaterialInstance _array_element "None" "None" :!class /Script/Engine.KismetMaterialLibrary))
    (Utilities|Array|AddUnique (Variables|Default|GetMaterialInstancesDynamic) _returnvalue)))

(fn SetMaterialtoDynamicInstances
  (for (_array_element _array_index) (Variables|Default|GetMaterialInstancesDynamic)
    (Rendering|Material|SetMaterial (Variables|Default|GetMesh) _array_index _array_element)))

(fn ResetMaterials
  (for (_array_element _array_index) (Variables|Default|GetOriginalMaterials)
    (Rendering|Material|SetMaterial (Variables|Default|GetMesh) _array_index _array_element)))

(fn FadeFinished
  (params (A :type Float%20%28double-precision%29))
  (if (>= A 1.0)
    (CallFunction|ResetMaterials)
    (if (Variables|Default|GetBlockVisibility)
      (Collision|SetCollisionResponsetoChannel (Variables|Default|GetMesh) "ECC_Visibility" "ECR_Block"))
    (elif (<= A 0.0)
      (if (Variables|Default|GetBlockVisibility)
        (Collision|SetCollisionResponsetoChannel (Variables|Default|GetMesh) "ECC_Visibility" "ECR_Ignore")))))